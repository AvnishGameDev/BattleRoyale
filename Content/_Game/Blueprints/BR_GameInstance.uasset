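; Game instance Blueprint that handles multiplayer matchmaking by joining an existing session or hosting a new one.
; TryJoinOrCreateGame destroys any current session, searches for games (LAN optional), and joins the first result through JoinSessionBP.
; If none is found or the search fails, it creates a session and opens FirstPersonExampleMap as a listen server.
; Successful hosting or joining enables the mouse cursor and Game and UI input; failures print errors.
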(event Custom|TryJoinOrCreateGame
  (bind _returnvalue (Game|GetPlayerController 0))
  (bind _returnvalue_2 (Game|GetPlayerController 0))
  (|DestroySession _returnvalue
    (:OnSuccess
      _)
    (:OnFailure
      _))
  (bind _results (|FindSessions _returnvalue 20 (Variables|Default|GetbUseLAN))
    (:OnSuccess
      (if (Utilities|Array|IsValidIndex _results)
        (CallFunction|JoinSessionBP (Utilities|Array|Get(acopy) _results))
        (else
          (|Session (Game|GetPlayerController 0) 20 (Variables|Default|GetbUseLAN) :!label _label
            (:OnSuccess
              (Game|OpenLevel(byName) "FirstPersonExampleMap" true "?listen")
              (Variables|/Script/Engine.PlayerController|SetbShowMouseCursor _returnvalue_2 true)
              (Input|SetInputModeGameandUI _returnvalue_2 0 "DoNotLock" true))
            (:OnFailure
              (Development|PrintString "Error creating session"))))))
    (:OnFailure
      (goto _label))))

(event Custom|JoinSessionBP
  (params (Session :type Blueprint%20Session%20Result%20Structure))
  (bind _returnvalue (Game|GetPlayerController 0))
  (|JoinSession (Game|GetPlayerController 0) Session
    (:OnSuccess
      (Variables|/Script/Engine.PlayerController|SetbShowMouseCursor _returnvalue true)
      (Input|SetInputModeGameandUI _returnvalue 0 "DoNotLock" true))
    (:OnFailure
      (Development|PrintString "Error Joining session"))))