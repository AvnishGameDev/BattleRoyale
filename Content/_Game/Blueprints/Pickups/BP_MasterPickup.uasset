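; BP_MasterPickup is a base pickup actor with a spinning mesh and a sphere that detects characters.
; Tick yaws the mesh steadily and zeroes its world pitch and roll, keeping it upright.
; Sphere overlaps with a BR_Character call empty PickupSphereEntered and PickupSphereLeft events, apparently hooks for child pickups.
; The sphere stops simulating physics on its first hit, so a physics-driven pickup freezes on contact.
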(event OnComponentBeginOverlap(PickupSphere)
  (params (OverlappedComponent :type Primitive%20Component%20Object%20Reference) (OtherActor :type Actor%20Object%20Reference) (OtherComp :type Primitive%20Component%20Object%20Reference) (OtherBodyIndex :type Integer) (bFromSweep :type Boolean) (SweepResult :type Hit%20Result%20Structure%20%28by%20ref%29))
  (bind _asbr_character (Utilities|Casting|CastToBR_Character OtherActor))
  (CallFunction|PickupSphereEntered _asbr_character))

(event OnComponentEndOverlap(PickupSphere)
  (params (OverlappedComponent :type Primitive%20Component%20Object%20Reference) (OtherActor :type Actor%20Object%20Reference) (OtherComp :type Primitive%20Component%20Object%20Reference) (OtherBodyIndex :type Integer))
  (bind _asbr_character (Utilities|Casting|CastToBR_Character OtherActor))
  (CallFunction|PickupSphereLeft _asbr_character))

(event OnComponentHit(PickupSphere)
  (params (HitComponent :type Primitive%20Component%20Object%20Reference) (OtherActor :type Actor%20Object%20Reference) (OtherComp :type Primitive%20Component%20Object%20Reference) (NormalImpulse :type Vector :default "0, 0, 0") (Hit :type Hit%20Result%20Structure%20%28by%20ref%29))
  (Physics|SetSimulatePhysics (Variables|Default|GetPickupSphere) false))

(event Custom|PickupSphereEntered
  (params (Character :type BR%20Character%20Object%20Reference)))

(event Custom|PickupSphereLeft
  (params (Character :type BR%20Character%20Object%20Reference)))

(event EventBeginPlay)

(event Collision|EventActorBeginOverlap
  (params (OtherActor :type Actor%20Object%20Reference)))

(event EventTick
  (params (DeltaSeconds :type Float%20%28single-precision%29))
  (bind _pickupmesh (Variables|Default|GetPickupMesh))
  (Transformation|AddRelativeRotation _pickupmesh (Math|Rotator|MakeRotator 0.0 0.0 (* DeltaSeconds 1.8e+02)) false false)
  (Transformation|SetWorldRotation (Variables|Default|GetPickupMesh) (Math|Rotator|MakeRotator 0.0 0.0 (.yaw (Transformation|GetWorldRotation _pickupmesh))) false false))

(fn ConstructionScript)