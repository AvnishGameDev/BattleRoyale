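; Weapon pickup actor that offers a weapon, with its clip and spare ammo, to characters inside its pickup sphere.
; On BeginPlay the authority fills both ammo counts from the weapon class defaults, unless the pickup was dropped by a player.
; Sphere enter and leave events set or clear the character's current weapon pickup reference, clearing it only if it still points to this pickup.
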(event EventBeginPlay
  (bind _weapontogive (Variables|Default|GetWeaponToGive))
  (bind (_damage _weaponname _currentammo _currentspareammo) (Utilities|GetClassDefaults _weapontogive))
  (Networking|SwitchHasAuthority
    (:Authority
      (if (not (Variables|Default|GetbDroppedByPlayer))
        (Variables|Default|SetCurrentAmmoInClip _currentammo)
        (Variables|Default|SetCurrentSpareAmmo _currentspareammo)))))

(event Collision|EventActorBeginOverlap
  (params (OtherActor :type Actor%20Object%20Reference)))

(event EventTick
  (params (DeltaSeconds :type Float%20%28single-precision%29)))

(event EventPickupSphereEntered
  (params (Character :type BR%20Character%20Object%20Reference))
  (Variables|/Game/FirstPersonBP/Blueprints/BR_Character.BR_Character_C|SetCurrentWeaponPickup Character self))

(event EventPickupSphereLeft
  (params (Character :type BR%20Character%20Object%20Reference))
  (if (== (Variables|/Game/FirstPersonBP/Blueprints/BR_Character.BR_Character_C|GetCurrentWeaponPickup Character) self)
    (Variables|/Game/FirstPersonBP/Blueprints/BR_Character.BR_Character_C|SetCurrentWeaponPickup Character 0)))

(fn ConstructionScript
  (|CallParentFunction))