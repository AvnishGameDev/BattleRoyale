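; BP_MasterWeapon is a weapon Blueprint that tracks clip and spare ammo for its BR_Character owner, cached at BeginPlay.
; Firing, ammo pickup and owner caching run only on the authority.
; OnFire decrements the clip and triggers Reload when empty, which flags the owner as reloading during a delay, then refills from spare ammo.
; GiveAmmo fills the clip before adding overflow to capped spare ammo; HasAmmo reports whether rounds remain.
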(event Custom|GiveAmmo
  (params (AmmoToGive :type Integer))
  ;[1 1 1] Add Ammo
  (Networking|SwitchHasAuthority
    (:Authority
      (Variables|Ammo|SetCurrentAmmo (+ (Variables|Ammo|GetCurrentAmmo) (Math|Integer|Min(Integer) (- (Variables|Ammo|GetClipSize) (Variables|Ammo|GetCurrentAmmo)) AmmoToGive)))
      (if (> (- AmmoToGive (Math|Integer|Min(Integer) (- (Variables|Ammo|GetClipSize) (Variables|Ammo|GetCurrentAmmo)) AmmoToGive)) 0)
        (Variables|Ammo|SetCurrentSpareAmmo (+ (Variables|Ammo|GetCurrentSpareAmmo) (Math|Integer|Min(Integer) (- AmmoToGive (Math|Integer|Min(Integer) (- (Variables|Ammo|GetClipSize) (Variables|Ammo|GetCurrentAmmo)) AmmoToGive)) (- (Variables|Ammo|GetMaxSpareAmmo) (Variables|Ammo|GetCurrentSpareAmmo)))))))))

(event Custom|OnFire
  (bind _currentammo (Variables|Ammo|GetCurrentAmmo))
  ;[1 1 1] On Fire
  (Networking|SwitchHasAuthority
    (:Authority
      (Math|Integer|DecrementInt _currentammo
        (:%20%20
          (if (<= _currentammo 0)
            (CallFunction|Reload)))))))

(event Custom|Reload
  ;[1 1 1] Reload
  (Variables|/Game/FirstPersonBP/Blueprints/BR_Character.BR_Character_C|SetbReloading (Variables|Default|GetCurrentOwner) true)
  (Utilities|FlowControl|Delay 2.0)
  (Variables|Ammo|SetCurrentAmmo (Math|Integer|Min(Integer) (Variables|Ammo|GetCurrentSpareAmmo) (Variables|Ammo|GetClipSize)))
  (Variables|Ammo|SetCurrentSpareAmmo (Math|Integer|Max(Integer) (- (Variables|Ammo|GetCurrentSpareAmmo) (Math|Integer|Min(Integer) (Variables|Ammo|GetCurrentSpareAmmo) (Variables|Ammo|GetClipSize)))))
  (Variables|/Game/FirstPersonBP/Blueprints/BR_Character.BR_Character_C|SetbReloading (Variables|Default|GetCurrentOwner) false))

(event EventBeginPlay
  ;[1 1 1] BeginPlay
  (Networking|SwitchHasAuthority
    (:Authority
      (bind _asbr_character (Utilities|Casting|CastToBR_Character (Components|GetOwner)))
      (Variables|Default|SetCurrentOwner _asbr_character))))

(event Collision|EventActorBeginOverlap
  (params (OtherActor :type Actor%20Object%20Reference)))

(event EventTick
  (params (DeltaSeconds :type Float%20%28single-precision%29)))

(fn ConstructionScript)

(fn HasAmmo
  (return (> (Variables|Ammo|GetCurrentAmmo) 0)))